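; Game mode Blueprint for Toon Tanks that handles the start and end of a match on screen.
; The StartGame event creates the start widget and adds it to the viewport.
; The GameOver event shows an end widget with win or loss text based on its WonGame input, then reopens the current level after a short delay.
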(event `self.StartGame`
  (bind _returnvalue (`|CreateWidget` "/Game/Blueprints/Widgets/WBP_StartGameWidget.WBP_StartGameWidget_C"))
  (`UserWidget.AddToViewport` _returnvalue 0))

(event `self.GameOver`
  (params (bWonGame :type Boolean))
  (bind _returnvalue (`|CreateWidget` "/Game/Blueprints/Widgets/WBP_EndGameWidget.WBP_EndGameWidget_C"))
  (`UserWidget.AddToViewport` _returnvalue 0)
  (`TextBlock.SetText` (`/Game/Blueprints/Widgets/WBP_EndGameWidget.DisplayText` _returnvalue) (`KismetTextLibrary.Conv_StringToText` (select `bool` bWonGame :`false` "YOU LOST!" :`true` "YOU WON!")))
  (bind _returnvalue_2 (`GameplayStatics.GetCurrentLevelName` true))
  (`KismetSystemLibrary.Delay` 4.0)
  (`GameplayStatics.OpenLevel` (`KismetStringLibrary.Conv_StringToName` _returnvalue_2)))

(fn `UserConstructionScript`)